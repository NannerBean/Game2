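; Stealth-game enemy character that patrols, investigates noises such as thrown rocks, chases the player and attacks in melee.
; Tick picks chase or waypoint/random patrol using visibility and a CanMove gate around AIMoveTo.
; PawnSensing sets visibility, triggers alert sound and chase music, and uses a retriggerable delay to lose sight.
; A montage notify runs the attack's sphere trace, which reloads the player's checkpoint on a hit.
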(event OnSeePawn(PawnSensing)
  (params (Pawn :type Pawn%20Object%20Reference))
  ;[0.15 0.07815 0.0278 0.5] Sets Visibilty
  (Utilities|FlowControl|Sequence
    (:then_0
      (Utilities|Casting|CastToBP_ThirdPersonCharacterCustom Pawn)
      (Development|PrintString "Hey! You stop right there!")
      (Variables|Default|SetbPlayerVisible true)
      (CallFunction|Alert)
      (Utilities|FlowControl|Delay 1.5)
      (Variables|Default|GetChaseMusic
        (:then)
        (:else
          (bind _returnvalue (Audio|SpawnSound2D "/Game/StealthGame/Effects/Sounds/CHASECcue.CHASECcue" 0.5 1.0 0.0 0))
          (Variables|Default|SetChaseMusic _returnvalue))))
    (:then_1
      (Utilities|FlowControl|RetriggerableDelay 0.2)
      (Development|PrintString "Must have been the wind...")
      (Variables|Default|SetbPlayerVisible false))))

(event OnHearNoise(PawnSensing)
  (params (Instigator :type Pawn%20Object%20Reference) (Location :type Vector%20%28by%20ref%29 :default "0, 0, 0") (Volume :type Float%20%28single-precision%29))
  ;[0.15 0.06378 0.1002 0.5] Get Distracted by Rock
  (CallFunction|UpdateWalkSpeed 5e+02)
  (Variables|Default|SetbCanMove false)
  (AI|AIMoveTo self Location Instigator 5e+01 false
    (:OnSuccess
      (Utilities|FlowControl|Delay 6.0)
      (Variables|Default|SetbCanMove true))))

(event Custom|ChasePlayer
  ;[0.15 0.1204 0.04023 0.5] Updates run speed and begins chase
  (CallFunction|UpdateWalkSpeed 5e+02)
  (Variables|Default|SetbCanMove false)
  (AI|AIMoveTo self "0, 0, 0" (Game|GetPlayerCharacter 0) 35.0 false
    (:OnSuccess
      (CallFunction|Attack)
      (Utilities|FlowControl|Delay 3.0)
      (Variables|Default|SetbCanMove true))))

(event Custom|PatrolRandom
  ;[0.1188 0.05401 0.15 0.5] Random Patrol
  (CallFunction|UpdateWalkSpeed 2e+02)
  (Variables|Default|SetbCanMove false)
  (AI|AIMoveTo self (.RandomLocation (AI|Navigation|GetRandomReachablePointinRadius (Transformation|GetActorLocation) 2e+03 0 0)) 0 5e+01 false
    (:OnSuccess
      (Utilities|FlowControl|Delay 3.0)
      (Variables|Default|SetbCanMove true))))

(event Custom|SetNextControlPointIndex
  ;[0.0237 0.15 0.1147 0.5] Sets which point to go to
  (Variables|Default|SetPatrolTargetPointIndex (Math|Integer|%(Integer) (+ (Variables|Default|GetPatrolTargetPointIndex) 1) (Utilities|Array|Length (Variables|Default|GetPatrolTargetPoints)))))

(event Custom|MoveToNextPatrolPoint
  ;[0.1287 0.15 0.05475 0.5] Tells enemy to move to next patrol point
  (CallFunction|UpdateWalkSpeed 3e+02)
  (Variables|Default|SetbCanMove false)
  (AI|AIMoveTo self "0, 0, 0" (Utilities|Array|Get(acopy) (Variables|Default|GetPatrolTargetPoints) (Variables|Default|GetPatrolTargetPointIndex)) 5e+01 false
    (:OnSuccess
      (Utilities|FlowControl|Delay 3.0)
      (Variables|Default|SetbCanMove true)
      (CallFunction|SetNextControlPointIndex))))

(event Custom|Alert
  (if (not (Variables|Default|GetbDidAlertPlay))
    (Variables|Default|SetbDidAlertPlay true)
    (Audio|PlaySoundatLocation "/Game/StealthGame/Effects/Sounds/676326__silverillusionist__horror-sting-apollyon-4.676326__silverillusionist__horror-sting-apollyon-4" (Transformation|GetActorLocation) "0, 0, 0" 0.5 1.0 0.0 0 0 0 0)))

(event Custom|Attack
  (bind _mesh (Variables|Character|GetMesh))
  (bind _returnvalue (Transformation|GetSocketLocation _mesh "hand_r"))
  ;[0.15 0.1407 0.04319 0.5] Bonk
  (Utilities|FlowControl|DoOnce false ; Only Reset Attack on miss.
    (:Completed
      (bind _notifyname (Animation|Montage|PlayMontage (Variables|Character|GetMesh) "/Game/StealthGame/Characters/Enemies/EnemyAI/AM_Attack_01.AM_Attack_01") ; Play the AM_Attack_01
        (:OnCompleted
          (if (Variables|Default|GetbHostile)
            (CallFunction|ResetAttack)))
        (:OnNotifyBegin
          (switch name _notifyname ; Pick the proper attack type(standard when there is more than one type of attack)
            (:AttackDamage
              (Development|PrintString "I'm attacking!")
              (bind (_outhits _returnvalue_2) (Collision|MultiSphereTraceForObjects _returnvalue (+ _returnvalue (* (Transformation|GetActorForwardVector) (Variables|Default|GetMeleeTraceDistance))) (Variables|Default|GetMeleeTraceRadius) (Utilities|Array|MakeArray "ObjectTypeQuery3") false 0 "None")) ; Trace forward from hand socket.
              (if _returnvalue_2 ; If a pawn is hit in that trace...
                (for _array_element _outhits ; ...loop through the results....
                  (bind _asbp_third_person_character_custom (Utilities|Casting|CastToBP_ThirdPersonCharacterCustom (.HitActor (Collision|BreakHitResult _array_element))))
                  (Default|LoadCheckpoint _asbp_third_person_character_custom)
                  (Variables|Default|SetbHostile false) ; ...and stop attacking...
                )))))))))

(event Custom|Reset%20Attack
  (bind _mesh (Variables|Character|GetMesh))
  (bind _returnvalue (Transformation|GetSocketLocation _mesh "hand_r"))
  ;[0.15 0.1407 0.04319 0.5] Bonk
  (Utilities|FlowControl|DoOnce false) ; enters at Reset
)

(event EventBeginPlay
  (bind _returnvalue (Actor|GetActorOfClass "/Script/Engine.PostProcessVolume"))
  (Variables|Default|SetPPV%20Ref _returnvalue))

(event Collision|EventActorBeginOverlap
  (params (OtherActor :type Actor%20Object%20Reference)))

(event EventTick
  (params (DeltaSeconds :type Float%20%28single-precision%29))
  (bind _bplayervisible (Variables|Default|GetbPlayerVisible))
  ;[0.15 0.02256 0.02657 0.5] Checks Enemy Status and acts accordingly
  (if (Variables|Default|GetbCanMove)
    (if _bplayervisible
      (CallFunction|ChasePlayer)
      (else
        (if (Variables|Default|GetbTargetPointMovement)
          (CallFunction|MovetoNextPatrolPoint)
          (else
            (CallFunction|PatrolRandom)))
        (bind _chasemusic (Variables|Default|GetChaseMusic)
          (:then
            (Audio|Components|Audio|FadeOut _chasemusic 3.0 0.0 "Linear" :!class /Script/Engine.AudioComponent)
            (Variables|Default|SetbDidAlertPlay false))
          (:else))))
    (elif _bplayervisible
      (CallFunction|ChasePlayer))))

(fn ConstructionScript)

(fn UpdateWalkSpeed
  (params (NewWalkSpeed :type Float%20%28double-precision%29))
  (Variables|/Script/Engine.CharacterMovementComponent|SetMaxWalkSpeed (Variables|Character|GetCharacterMovement) NewWalkSpeed))